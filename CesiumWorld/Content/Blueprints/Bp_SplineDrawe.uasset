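; Spline drawer actor that, as wired, only resets its spline when play begins.
; BeginPlay clears the spline points and loops over SplineMeshActors destroying entries, but empties the array inside the loop body, so only the first gets destroyed.
; An unconnected chain would rebuild the spline as two world-space points at the Marker1Ref and Marker2Ref locations.
; The construction script is empty, and no spline meshes are created here.
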(event `self.ReceiveBeginPlay`
  (`SplineComponent.ClearSplinePoints` (`self.Spline`) true)
  (for _array_element (`self.SplineMeshActors`)
    (`ActorComponent.K2_DestroyComponent` _array_element)
    (`KismetArrayLibrary.Array_Clear` (`self.SplineMeshActors`))))

(fn `UserConstructionScript`)