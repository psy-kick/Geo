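; Player control Blueprint for mouse-driven dragging of actors tagged "Draggable".
; BeginPlay enables the cursor, click and hover events with Game and UI input.
; Left click traces under the cursor, prints the hit actor's name and sets IsDragging from its tag.
; While set, Tick re-traces and moves whichever actor is hit to its location minus the hit point; no release handler clears the flag.
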(event `self.ReceiveBeginPlay`
  (`WidgetBlueprintLibrary.SetInputMode_GameAndUIEx` (`GameplayStatics.GetPlayerController` 0) null "DoNotLock" false)
  (set `self.bShowMouseCursor` true)
  (set `self.bEnableMouseOverEvents` true)
  (set `self.bEnableClickEvents` true))

(event `Key|LeftMouseButton`
  (params (Key :type "Key Structure"))
  (bind (_bblockinghit _binitialoverlap _time _distance _location _impactpoint _normal _impactnormal _physmat _hitactor) (`GameplayStatics.BreakHitResult` (`self.GetHitResultUnderCursorByChannel` "TraceTypeQuery1")))
  (:`Pressed`
    (set `self.isDragging` true)
    (set `self.isDragging` (`self.ActorHasTag` _hitactor "Draggable"))
    (`KismetSystemLibrary.PrintString` (`KismetSystemLibrary.GetDisplayName` _hitactor))))

(event `OnClicked_Event`
  (params (TouchedActor :type "Actor Object Reference") (ButtonPressed :type "Key Structure" :default "None")))

(event `self.ReceiveTick`
  (params (DeltaSeconds :type "Float (single-precision)"))
  (bind (_bblockinghit _binitialoverlap _time _distance _location _impactpoint _normal _impactnormal _physmat _hitactor) (`GameplayStatics.BreakHitResult` (`self.GetHitResultUnderCursorByChannel` "TraceTypeQuery1")))
  (if (`self.isDragging`)
    (bind _output_get (set `self.Hit Actor` _hitactor))
    (`self.K2_SetActorLocation` _output_get (- (`self.K2_GetActorLocation` _hitactor) _location) false false)))

(fn `UserConstructionScript`)