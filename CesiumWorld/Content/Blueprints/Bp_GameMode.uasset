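; Game mode that sets up the HUD and an opening popup shortly after play begins.
; After a brief delay, it has the HUD manager create a message, show the compass message and register the game mode itself as a screen-persistent compass marker with manual distance info.
; It then creates a UIPopup widget for the first player and adds it to the viewport.
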(event `self.ReceiveBeginPlay`
  (`KismetSystemLibrary.Delay` 0.2)
  (message `/Game/ProHUDV2_NavOnly/Blueprints/Libraries/BPi_HUDManagerV2_N.CreateHUD` (`KismetSystemLibrary.Conv_InterfaceToObject` (`/Game/ProHUDV2_NavOnly/Blueprints/Libraries/BP_PHV2_Functions_N.GetHUDManager`)) 0)
  (message `/Game/ProHUDV2_NavOnly/Blueprints/Libraries/BPi_HUDManagerV2_N.ShowCompass` (`KismetSystemLibrary.Conv_InterfaceToObject` (`/Game/ProHUDV2_NavOnly/Blueprints/Libraries/BP_PHV2_Functions_N.GetHUDManager`)))
  (`/Game/ProHUDV2_NavOnly/Blueprints/Libraries/BPi_HUDManagerV2_N.AddOrUpdateCompassMarker` (`/Game/ProHUDV2_NavOnly/Blueprints/Libraries/BP_PHV2_Functions_N.GetHUDManager`) self (make `/Game/ProHUDV2_NavOnly/Blueprints/Structs/S_CompassMarkerInfo_N` null 1.0 (struct) (struct) false false (make `/Game/ProHUDV2_NavOnly/Blueprints/Structs/S_TextInfo_N` false (struct :`OutlineSettings` (struct :`OutlineColor` (struct :`A` 1.0)) :`Size` 24.0 :`MonospacedWidth` 1.0) 1.0 (struct :`R` 1.0 :`G` 1.0 :`B` 1.0 :`A` 1.0)) (make `/Game/ProHUDV2_NavOnly/Blueprints/Structs/S_DistanceInfo_N` true) 0 true true))
  (bind _returnvalue (`|CreateWidget` "/Game/Blueprints/UIPopup.UIPopup_C" (`GameplayStatics.GetPlayerController` 0)))
  (`UserWidget.AddToViewport` _returnvalue 0))

(fn `UserConstructionScript`)